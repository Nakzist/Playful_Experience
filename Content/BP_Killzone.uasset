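; BP_Killzone is a recycled hazard with a randomized mesh that reloads the current level when the player character overlaps it.
; A fast looping timer checks whether the player has passed it along X.
; Once passed, it waits briefly, then leapfrogs a fixed distance ahead and picks one of three Y lanes at random, so it repeats endlessly.
; The construction script picks the Cube component's mesh from an array.
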(event Custom|CustomEvent
  (bind _returnvalue (Transformation|GetActorLocation))
  (bind _returnvalue_2 (+ _returnvalue "12000.000000,0.000000,0.000000"))
  (if (> (.x (Transformation|GetActorLocation (Variables|Default|GetAs%20BP%20Third%20Person%20Character))) (.x (Transformation|GetActorLocation)))
    (Utilities|FlowControl|Delay 2.0)
    (Transformation|SetActorLocation (Math|Vector|MakeVector (.x _returnvalue_2) (Math|Conversions|ToFloat(Integer) (* (Math|Random|RandomIntegerinRange -1 1) 100)) (.z _returnvalue_2)) false false)))

(event EventBeginPlay
  (bind _asbp_third_person_character (Utilities|Casting|CastToBP_ThirdPersonCharacter (Game|Player|GetPlayerPawn 0)))
  (Variables|Default|SetAs%20BP%20Third%20Person%20Character _asbp_third_person_character)
  (Utilities|Time|SetTimerbyEvent (delegate Custom|CustomEvent) 0.025 true))

(event Collision|EventActorBeginOverlap
  (params (OtherActor :type Actor%20Object%20Reference))
  (Utilities|Casting|CastToBP_ThirdPersonCharacter OtherActor)
  (bind _returnvalue (Game|GetCurrentLevelName true))
  (Game|OpenLevel(byName) (Utilities|String|StringToName _returnvalue)))

(event EventTick
  (params (DeltaSeconds :type Float%20%28single-precision%29)))

(fn ConstructionScript
  (Components|StaticMesh|SetStaticMesh (Variables|Default|GetCube) (.OutItem (Utilities|Array|Random (Variables|Default|Getstaticmesh)))))